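; BP_LobbyPlayerCtroller is the player controller for the lobby screen.
; On BeginPlay, for a local controller outside a dedicated server, it creates the WBP_Lobby widget, adds it to the viewport, stores it and shows the mouse cursor.
; RebuildPlayerList forwards to the stored widget's function of the same name when that widget is valid.
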(event `self.ReceiveBeginPlay`
  (bind _returnvalue (`GameplayStatics.GetPlayerController` 0))
  (if (and (not (`KismetSystemLibrary.IsDedicatedServer`)) (`self.IsLocalController`))
    (bind _returnvalue_2 (`|CreateWidget` "/Game/Blueprint/WBP_Lobby.WBP_Lobby_C" _returnvalue))
    (`UserWidget.AddToViewport` _returnvalue_2 0)
    (set `self.LobbyWidget` _returnvalue_2)
    (set `PlayerController.bShowMouseCursor` true _returnvalue)))

(event `self.ReceiveTick`
  (params (DeltaSeconds :type "Float (single-precision)")))

(fn `Rebuild Player List`
  (bind _lobbywidget (`self.LobbyWidget`))
  (`/Engine/EditorBlueprintResources/StandardMacros.IsValid` _lobbywidget
    (:`Is Valid`
      (`/Game/Blueprint/WBP_Lobby.RebuildPlayerList` _lobbywidget))))

(fn `UserConstructionScript`)