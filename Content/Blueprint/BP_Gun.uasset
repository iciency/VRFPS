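; Gun actor that handles the firing presentation for an owning character, with no hit or projectile logic in this graph.
; OnFire plays shoot montages on the gun mesh and the owner's body and arm meshes, plus an M4A1 shot sound at the muzzle.
; Debug helpers print owner cast results on BeginPlay and draw a red line along the actor's right vector each tick.
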(event `self.ReceiveBeginPlay`
  (bind _asbase_character (cast `BaseCharacter` (`self.GetOwner`)))
  (`KismetSystemLibrary.PrintString` (`KismetSystemLibrary.GetObjectName` _asbase_character))
  (cast `/Game/Blueprint/BP_BaseCharacter` (`self.GetOwner`)
    (:`then`
      (`KismetSystemLibrary.PrintString` "Hello"))
    (:`CastFailed`
      (`KismetSystemLibrary.PrintString` "fa"))))

(event `self.ReceiveTick`
  (params (DeltaSeconds :type "Float (single-precision)"))
  (bind _returnvalue (`self.K2_GetActorLocation`))
  (`KismetSystemLibrary.DrawDebugLine` _returnvalue (+ (* (`self.GetActorRightVector`) 1000.0) _returnvalue) (struct :`R` 1.0 :`A` 1.0)))

(event `self.OnFire`
  (`|ExecutionSequence`
    (:`then_0`
      (`|PlayMontage` (`self.SkeletalMesh`) "/Game/FPS_Assault_Pack/Animations/Rifle/A_Rifle_Shoot01_Montage.A_Rifle_Shoot01_Montage"
        (:`then`
          (bind _asbp_base_character (cast `/Game/Blueprint/BP_BaseCharacter` (`self.GetOwner`)))
          (`|PlayMontage` (`Character.Mesh` _asbp_base_character) "/Game/AnimStarterPack/Fire_Rifle_Hip_Montage.Fire_Rifle_Hip_Montage"
            (:`then`
              (`|PlayMontage` (`/Game/Blueprint/BP_BaseCharacter.ArmMesh` _asbp_base_character) "/Game/FPS_Assault_Pack/Animations/Rifle/A_Arms_Rifle_Shoot01_Montage.A_Arms_Rifle_Shoot01_Montage"))))))
    (:`then_1`
      (`GameplayStatics.SpawnSoundAtLocation` "/Game/m4a1_unsil-1.m4a1_unsil-1" (`self.GetMuzzleLocation`) (struct) 1.0 1.0 0.0 null null))))

(fn `UserConstructionScript`)