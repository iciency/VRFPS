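; Game mode for the VR gun deathmatch that holds players in a waiting state until at least two have joined.
; On PostLogin it copies the game instance's VR flag to the player state, puts the first player on team 0 and later ones on team 1, then calls AwakePlay.
; Once the count reaches two, GameStart removes each player's wait UI and spawns their character.
; BeginPlay only prints debug messages.
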(event `self.K2_PostLogin`
  (params (NewPlayer :type "PlayerController Object Reference"))
  (bind _asbp_game_instance (cast `/Game/Blueprint/BP_GameInstance` (`GameplayStatics.GetGameInstance`)))
  (`KismetArrayLibrary.Array_Add` (`self.PlayerList`) NewPlayer)
  (bind _asbp_vrgun_player_state (cast `/Game/Blueprint/BP_VRGunPlayerState` (`Controller.PlayerState` NewPlayer)))
  (set `/Game/Blueprint/BP_VRGunPlayerState.VR` (`/Game/Blueprint/BP_GameInstance.UseVR` _asbp_game_instance) _asbp_vrgun_player_state)
  (if (== (`self.PlayerCount`) 0)
    (set `/Game/Blueprint/BP_VRGunPlayerState.Team` 0 _asbp_vrgun_player_state)
    (else
      (set `/Game/Blueprint/BP_VRGunPlayerState.Team` 1 _asbp_vrgun_player_state)))
  (`/Game/Blueprint/BP_VRGunPlayerState.AwakePlay` _asbp_vrgun_player_state NewPlayer)
  (`/Engine/EditorBlueprintResources/StandardMacros.IncrementInt` (`self.PlayerCount`)
    (:`  `
      (if (>= (`self.PlayerCount`) 2)
        (`self.GameStart`)))))

(event `self.ReceiveBeginPlay`
  (`KismetSystemLibrary.PrintString` "mapBegin" true true (struct :`R` 0.051854 :`G` 0.14052 :`B` 1.0 :`A` 1.0) 10.0)
  (bind _asbp_game_instance (cast `/Game/Blueprint/BP_GameInstance` (`GameplayStatics.GetGameInstance`))
    (:`then`
      (`KismetSystemLibrary.PrintString` (`KismetStringLibrary.Conv_BoolToString` (`/Game/Blueprint/BP_GameInstance.UseVR` _asbp_game_instance)) true true (struct :`G` 1.0 :`B` 0.217914 :`A` 1.0) 10.0))
    (:`CastFailed`
      (`KismetSystemLibrary.PrintString` "Instance  cast faild" true true (struct :`R` 1.0 :`G` 0.141862 :`A` 1.0) 10.0))))

(event `self.ReceiveTick`
  (params (DeltaSeconds :type "Float (single-precision)")))

(event `GameStart`
  (for _array_element (`self.PlayerList`)
    (bind _playerstate (`Controller.PlayerState` _array_element))
    (bind _asbp_vrgun_player_state (cast `/Game/Blueprint/BP_VRGunPlayerState` _playerstate))
    (`/Game/Blueprint/BP_VRGunPlayerState.RemoveWaitUI` _asbp_vrgun_player_state)
    (bind _asbp_base_character (cast `/Game/Blueprint/BP_BaseCharacter` (`PlayerState.PawnPrivate` _playerstate)))
    (`/Game/Blueprint/BP_BaseCharacter.Spawn` _asbp_base_character)))

(fn `UserConstructionScript`)