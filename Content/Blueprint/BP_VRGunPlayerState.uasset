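; BP_VRGunPlayerState is a player state for the VR gun game that manages each player's in-game waiting screen.
; AwakePlay creates WBP_InGameWait for the given player, adds it to the viewport and stores it.
; RemoveWaitUI runs a one-second Delay loop that increments CountDown, pushes it to the widget's text and removes the widget when the count reaches ten.
; Both events print debug strings.
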(event `AwakePlay`
  (params (Player :type "PlayerController Object Reference"))
  (`KismetSystemLibrary.PrintString` "wat" true true (struct :`R` 0.343419 :`G` 1.0 :`B` 0.542752 :`A` 1.0) 12.0)
  (bind _returnvalue (`|CreateWidget` "/Game/Blueprint/WBP_InGameWait.WBP_InGameWait_C" Player))
  (`UserWidget.AddToViewport` _returnvalue 0)
  (set `self.WaitWidget` _returnvalue))

(event `RemoveWaitUI`
  (bind _waitwidget (`self.WaitWidget`))
  (bind _countdown (`self.CountDown`))
  (`KismetSystemLibrary.PrintString` (`KismetStringLibrary.Conv_IntToString` _countdown) :!label _label)
  (`KismetSystemLibrary.Delay` 1.0)
  (bind _result (`/Engine/EditorBlueprintResources/StandardMacros.IncrementInt` _countdown)
    (:`  `
      (bind _aswbp_in_game_wait (cast `/Game/Blueprint/WBP_InGameWait` _waitwidget))
      (`/Game/Blueprint/WBP_InGameWait.SetText` _aswbp_in_game_wait _countdown)
      (if (== _result 10)
        (`Widget.RemoveFromParent` _waitwidget)
        (else
          (goto _label))))))

(fn `UserConstructionScript`)