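; Base character for a networked team shooter supporting VR and non-VR players.
; On weapon setup it teleports to a random start actor for the PlayerState's team, then configures the view.
; The weapon attaches to the motion controller, first-person arms or body mesh, with mesh visibility set by VR mode and local control.
; Death ragdolls the body, attaches the local camera to its head and runs ServerTravel to Lobby after a delay.
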(event `Spawn`
  (bind _returnvalue (`self.GetController` (`PawnMovementComponent.GetPawnOwner` (`self.CharacterMovement`))))
  (bind _asbp_vrgun_player_state (cast `/Game/Blueprint/BP_VRGunPlayerState` (`self.PlayerState`)))
  (if (== (`/Game/Blueprint/BP_VRGunPlayerState.Team` _asbp_vrgun_player_state) 0)
    (bind _outactors (`GameplayStatics.GetAllActorsOfClass` "/Game/Blueprint/BP_T1_Start.BP_T1_Start_C"))
    (bind _outitem (`KismetArrayLibrary.Array_Random` _outactors))
    (`self.K2_SetActorLocationAndRotation` (`self.K2_GetActorLocation` _outitem) (`self.K2_GetActorRotation` _outitem))
    (`Controller.SetControlRotation` _returnvalue (`KismetMathLibrary.MakeRotator` 0.0 0.0 -90.0))
    (`KismetSystemLibrary.PrintString` "Teleport" true true (struct :`R` 1.0 :`B` 0.119987 :`A` 1.0) 12.0)
    (else
      (bind _outactors_2 (`GameplayStatics.GetAllActorsOfClass` "/Game/Blueprint/BP_T2_Start.BP_T2_Start_C"))
      (bind _outitem_2 (`KismetArrayLibrary.Array_Random` _outactors_2))
      (`self.K2_SetActorLocationAndRotation` (`self.K2_GetActorLocation` _outitem_2) (`self.K2_GetActorRotation` _outitem_2))
      (`Controller.SetControlRotation` _returnvalue (`KismetMathLibrary.MakeRotator` 0.0 0.0 90.0))
      (`KismetSystemLibrary.PrintString` "Teleport" true true (struct :`R` 1.0 :`B` 0.119987 :`A` 1.0) 12.0))))

(event `self.ReceiveBeginPlay`
  (bind _returnvalue (`self.IsLocallyControlled`))
  (bind _weaponactor (`self.WeaponActor`))
  (bind _mesh (`self.Mesh`))
  (bind _armmesh (`self.ArmMesh`))
  (if (`self.IsLocallyControlled`)
    (`Controller.SetControlRotation` (`self.GetController` (`PawnMovementComponent.GetPawnOwner` (`self.CharacterMovement`))) (`KismetMathLibrary.MakeRotator` 0.0 0.0 90.0)))
  (bind _asbp_vrgun_player_state (cast `/Game/Blueprint/BP_VRGunPlayerState` (`self.PlayerState`) :!label _label)
    (:`then`
      (set `self.UseVR` (`/Game/Blueprint/BP_VRGunPlayerState.VR` _asbp_vrgun_player_state)))
    (:`CastFailed`
      _))
  (if (`self.UseVR`)
    (if _returnvalue
      (`self.K2_AttachToComponent` _weaponactor (`self.MotionController`) "None" "KeepRelative" "KeepRelative" "KeepRelative" true)
      (`SceneComponent.SetVisibility` (`self.Mesh`) false true)
      (`SceneComponent.SetVisibility` (`self.ArmMesh`) false true)
      (else
        (`KismetSystemLibrary.PrintString` "vr local" true true (struct :`G` 0.66 :`B` 1.0 :`A` 1.0) 5.0)
        (`self.K2_AttachToComponent` _weaponactor (`self.Mesh`) "R_GunSocket" "KeepRelative" "KeepRelative" "KeepRelative" true :!label _label_2)
        (`SceneComponent.SetVisibility` _mesh true true)
        (`SceneComponent.SetVisibility` _armmesh false true)))
    (elif _returnvalue
      (`self.K2_AttachToComponent` _weaponactor (`self.ArmMesh`) "R_GunSocket" "KeepRelative" "KeepRelative" "KeepRelative" true)
      (`SceneComponent.SetVisibility` _mesh false true)
      (`SceneComponent.SetVisibility` _armmesh true true)
      (else
        (goto _label_2)))))

(event `self.OnSetupWeapon`
  (`self.Spawn`)
  (goto _label))

(event `self.ReceiveTick`
  (params (DeltaSeconds :type "Float (single-precision)")))

(event `self.OnDie`
  (bind _mesh (`self.Mesh`))
  (`|ExecutionSequence`
    (:`then_0`
      (`SceneComponent.SetVisibility` _mesh true true)
      (`PrimitiveComponent.SetSimulatePhysics` _mesh true)
      (`PrimitiveComponent.SetCollisionEnabled` _mesh "QueryAndPhysics")
      (set `SkeletalMeshComponent.bPauseAnims` true _mesh)
      (`SceneComponent.SetVisibility` (`self.ArmMesh`) false true)
      (`KismetSystemLibrary.Delay` 3.0)
      (`self.GameEnd`))
    (:`then_1`
      (if (`self.IsLocallyControlled`)
        (`SceneComponent.K2_AttachToComponent` (`self.Camera`) (`self.Mesh`) "head" "SnapToTarget" "SnapToTarget" "KeepWorld" true)))))

(event `GameEnd`
  (bind _returnvalue (`GameplayStatics.GetPlayerController` 0))
  (if (!= (`self.GetController`) _returnvalue)
    (`KismetSystemLibrary.ExecuteConsoleCommand` "ServerTravel Lobby" _returnvalue)
    (else
      (`KismetSystemLibrary.ExecuteConsoleCommand` "ServerTravel Lobby" (`GameplayStatics.GetPlayerController` 1)))))

(fn `UserConstructionScript`)